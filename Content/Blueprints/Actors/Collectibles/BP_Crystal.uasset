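; BP_Crystal is a collectible crystal actor that gets pulled into the player when the player overlaps it.
; On overlap it stores its starting location, scale and point light intensity, then plays a collection timeline.
; Each update lerps it toward the player's current position while shrinking it to zero and fading its light.
; When the timeline finishes, the actor destroys itself.
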(event Collision|EventActorBeginOverlap
  (params (OtherActor :type Actor%20Object%20Reference))
  (Utilities|IsPlayer OtherActor
    (:Is%20Player
      (CallFunction|StoreStartingValues)
      (bind _collection_progress (Timeline|Collection%20Timeline Play)
        (:Update
          (CallFunction|MovetoPlayer _collection_progress)
          (CallFunction|ScaleCrystal _collection_progress)
          (CallFunction|ChangeLightIntensity _collection_progress))
        (:Finished
          (Actor|DestroyActor))))))

(fn ConstructionScript)

(fn MovetoPlayer
  (params (Alpha :type Float%20%28single-precision%29))
  (Transformation|SetActorLocation (Math|Vector|Lerp(Vector) (Variables|Default|GetStart%20Location) (Transformation|GetActorLocation (Game|Player|GetPlayerPawn 0)) Alpha) false false))

(fn StoreStartingValues
  (Variables|Default|SetStart%20Location (Transformation|GetActorLocation))
  (Variables|Default|SetStart%20Scale (Transformation|GetActorScale3D))
  (Variables|Default|SetStart%20Light%20Intensity (Variables|/Script/Engine.LightComponentBase|GetIntensity (Variables|Default|GetPointLight))))

(fn ScaleCrystal
  (params (Alpha :type Float%20%28single-precision%29))
  (Transformation|SetActorScale3D (Math|Vector|Lerp(Vector) (Variables|Default|GetStart%20Scale) "0, 0, 0" Alpha)))

(fn ChangeLightIntensity
  (params (Alpha :type Float%20%28single-precision%29))
  (Rendering|Components|Light|SetIntensity (Variables|Default|GetPointLight) (Math|Float|Lerp (Variables|Default|GetStart%20Light%20Intensity) 0.0 Alpha)))