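; BP_Cannon is an automatic cannon actor that repeatedly fires BP_Projectile on a FireRate delay, starting at BeginPlay.
; Each shot spawns a projectile at the ProjectileDirection component's transform, scaled by ProjectileSize, then plays the CannonFireAnimation timeline.
; The timeline moves the barrel along its relative Y axis, and its Update output loops back into the Delay to schedule the next shot.
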(event EventBeginPlay
  (Utilities|FlowControl|Delay (Variables|CannonProperties|GetFire%20Rate) :!label _label)
  (CallFunction|SpawnProjectile)
  (bind _cannon_barrel_location (Timeline|Cannon%20Fire%20Animation PlayFromStart)
    (:Update
      (CallFunction|MoveCannonBarrelYLocation _cannon_barrel_location)
      (goto _label))))

(fn ConstructionScript)

(fn SpawnProjectile
  (bind _projectile_direction (Variables|Default|GetProjectile%20Direction))
  (bind _returnvalue (Transformation|GetWorldTransform _projectile_direction))
  (Game|SpawnActorfromClass "/Game/Blueprints/Actors/Projectiles/BP_Projectile.BP_Projectile_C" (Math|Transform|MakeTransform (.location _returnvalue) (.rotation _returnvalue) (Math|Conversions|ToVector(Float) (Variables|CannonProperties|GetProjectile%20Size))) "Undefined" 0 0))

(fn MoveCannonBarrelYLocation
  (params (NewLocation_Y :type Float%20%28single-precision%29))
  (Transformation|SetRelativeLocation (Variables|Default|GetCannon%20Barrel) (Math|Vector|MakeVector 0.0 NewLocation_Y 0.0) false false))