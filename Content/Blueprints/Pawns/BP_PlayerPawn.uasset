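; Player pawn for a rolling ball that restarts the level when it takes any damage.
; Forward/back and left/right axis inputs share one torque call on the Sphere, applied as an acceleration change scaled by AccelerationFactor.
; The camera fades in on BeginPlay; Restart Level uses a DoOnce to fade out once, wait out the fade, then reopen the current level by name.
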(event EventBeginPlay
  (CameraFades|StartCameraFade :self (Game|GetPlayerCameraManager 0) :FromAlpha 1.0 :Duration (Math|Float|MakeLiteralFloat 1.0)))

(event Game|Damage|EventAnyDamage
  (params (Damage :type Float%20%28single-precision%29) (DamageType :type Damage%20Type%20Object%20Reference) (InstigatedBy :type Controller%20Object%20Reference) (DamageCauser :type Actor%20Object%20Reference))
  (Utilities|RestartLevel))

(event Input|AxisEvents|InputAxisForwardsandBackwards
  (params (AxisValue :type Float%20%28single-precision%29))
  (bind _acceleration_factor (Variables|Default|GetAcceleration%20Factor))
  (Class|PrimitiveComponent|AddTorqueinRadians (Variables|Default|GetSphere) (Math|Vector|MakeVector (* (stale Input|AxisEvents|InputAxisLeftandRight AxisValue) _acceleration_factor) (* AxisValue _acceleration_factor) 0.0) "None" true))

(event Input|AxisEvents|InputAxisLeftandRight
  (params (AxisValue :type Float%20%28single-precision%29))
  (bind _acceleration_factor (Variables|Default|GetAcceleration%20Factor))
  (Class|PrimitiveComponent|AddTorqueinRadians (Variables|Default|GetSphere) (Math|Vector|MakeVector (* AxisValue _acceleration_factor) (* (stale Input|AxisEvents|InputAxisForwardsandBackwards AxisValue) _acceleration_factor) 0.0) "None" true))

(fn ConstructionScript)